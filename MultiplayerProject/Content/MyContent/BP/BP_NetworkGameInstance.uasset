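; Game instance that hosts and joins LAN multiplayer sessions.
; CreateGame creates a session and opens the test level as a listen server, while JoinToGame joins a given search result.
; Both then wait a fixed delay before telling the local BP_MultiplayerPawn to create its health widget, rather than reacting to possession.
; Session search and server-list printing logic is present but disconnected, so it never runs.
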(event Custom|CreateGame
  (bind _returnvalue (Game|GetPlayerController 0))
  ;[1 1 1] Create Game
  (|Session _returnvalue 16 true
    (:OnSuccess
      (Game|OpenLevel(byName) "TestLevel" true "listen")
      (Utilities|FlowControl|Delay 2.0)
      (bind _asbp_multiplayer_pawn (Utilities|Casting|CastToBP_MultiplayerPawn (Pawn|GetControlledPawn _returnvalue)))
      (Default|CreateHealthWidgetonViewport _asbp_multiplayer_pawn))
    (:OnFailure
      (Development|PrintString "ouch! Game creation error!"))))

(event Custom|JoinToGame
  (params (SearchResult :type Blueprint%20Session%20Result%20Structure%20%28by%20ref%29))
  (bind _returnvalue (Game|GetPlayerController 0))
  (|JoinSession _returnvalue SearchResult
    (:then
      (Utilities|FlowControl|Delay 2.0)
      (bind _asbp_multiplayer_pawn (Utilities|Casting|CastToBP_MultiplayerPawn (Pawn|GetControlledPawn _returnvalue))
        (:then
          (Default|CreateHealthWidgetonViewport _asbp_multiplayer_pawn))
        (:CastFailed
          (Development|PrintString "Fail" true true "(R=1.000000,G=0.819077,B=0.000000,A=1.000000)"))))))