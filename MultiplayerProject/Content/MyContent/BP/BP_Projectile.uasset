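; BP_Projectile is a multiplayer projectile that flies forward, damages pawns and explodes on impact.
; The server moves it each Tick by setting location without sweep, while a BeginPlay timer destroys it when its lifetime ends.
; Sphere overlaps are resolved on the server, ignoring the owner and other projectiles.
; BP_MultiplayerPawn hits take damage and print health; any valid hit multicasts an explosion emitter, then destroys the projectile.
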(event OnComponentBeginOverlap(Sphere)
  (params (OverlappedComponent :type Primitive%20Component%20Object%20Reference) (OtherActor :type Actor%20Object%20Reference) (OtherComp :type Primitive%20Component%20Object%20Reference) (OtherBodyIndex :type Integer) (bFromSweep :type Boolean) (SweepResult :type Hit%20Result%20Structure%20%28by%20ref%29))
  ;[1 1 1] Пересечение снарядом чего нибудь
  (if (Networking|IsServer)
    (CallFunction|ServerCollision OtherActor (Transformation|GetActorLocation))))

(event Custom|LefeEnd
  ;[1 1 1] Projectile Life
  (CallFunction|ServerLifeEnded))

(event Custom|Server_Move
  (params (DeltaTime :type Float%20%28single-precision%29))
  ;[1 1 1] Move
  (Transformation|SetActorLocation (+ (Transformation|GetActorLocation) (* (Transformation|GetActorForwardVector) (* DeltaTime (Variables|Default|GetSpeed)))) false false))

(event Custom|Server_collision
  (params (OtherActor :type Actor%20Object%20Reference) (Location :type Vector))
  ;[1 1 1] Проверка на пересеччение
  (if (!= OtherActor (Components|GetOwner))
    (bind _asbp_multiplayer_pawn (Utilities|Casting|CastToBP_MultiplayerPawn OtherActor)
      (:then
        (Default|TakeDamage _asbp_multiplayer_pawn (Variables|Default|GetDamage) _asbp_multiplayer_pawn)
        (Development|PrintString (Utilities|String|ToString(Float) (Variables|/Game/MyContent/BP/HealthComponent.HealthComponent_C|GetCurrentHEalth (Variables|/Game/MyContent/BP/BP_MultiplayerPawn.BP_MultiplayerPawn_C|GetHealthComponent _asbp_multiplayer_pawn))) true true "(R=0.083954,G=1.000000,B=0.000000,A=1.000000)"))
      (:CastFailed
        (Utilities|Casting|CastToBP_Projectile OtherActor
          (:CastFailed
            _))))
    (CallFunction|MulticastHitEffect Location)
    (CallFunction|ServerLifeEnded)))

(event Custom|Server_LifeEnded
  ;[1 1 1] Projectile Life
  (Actor|DestroyActor))

(event Custom|Spawn%20Hit%20Effect
  (params (HitLocation :type Vector))
  ;[1 1 1] Effect
  (Effects|SpawnEmitteratLocation "/Game/StarterContent/Particles/P_Explosion.P_Explosion" HitLocation))

(event Custom|Multicast_HitEffect
  (params (Hit%20HitLOcation :type Vector))
  ;[1 1 1] Effect
  (CallFunction|SpawnHitEffect Hit%20HitLOcation))

(event EventBeginPlay
  ;[1 1 1] Projectile Life
  (Utilities|Time|SetTimerbyEvent (delegate Custom|LefeEnd) (Variables|Default|GetLifeTime)))

(event Collision|EventActorBeginOverlap
  (params (OtherActor :type Actor%20Object%20Reference)))

(event EventTick
  (params (DeltaSeconds :type Float%20%28single-precision%29))
  (if (Networking|IsServer)
    (CallFunction|ServerMove DeltaSeconds)))

(fn ConstructionScript)