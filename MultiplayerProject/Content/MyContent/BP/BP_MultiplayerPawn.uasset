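; Player pawn for a team multiplayer shooter, with movement, jumping, a team-colored name label and debug team printout.
; Team ID comes from the controller through a server event, then a multicast sets the sphere material.
; Server events spawn projectiles behind a Delay-based reload and subtract damage from HealthComponent, while Tick destroys the pawn at zero health.
; A key opens a pause widget and unpossesses; health widget creation exists but is never called.
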(event Custom|Server_Fire
  (bind _self self)
  (bind _arrow1 (Variables|Default|GetArrow1))
  (bind _returnvalue (Transformation|GetWorldTransform _arrow1))
  ;[1 0 0] Задержка выстрела/ Reload
  (if (Variables|Default|GetCanFire)
    ;[1 1 1] Server_Fire
    (Game|SpawnActorfromClass (Variables|Default|GetProjectileClass) (Math|Transform|MakeTransform (.location _returnvalue) (.rotation _returnvalue) (.scale _returnvalue)) "Undefined" _self _self)
    (CallFunction|Reload)))

(event Custom|TakeDamage
  (params (Damage%20Value :type Float%20%28single-precision%29) (MultiPawn :type BP%20Multiplayer%20Pawn%20Object%20Reference))
  ;[1 1 1] Damage
  (CallFunction|ServerTakeDamage Damage%20Value MultiPawn))

(event Custom|GeneratePlayerName
  (params (NumberInTeam :type Integer))
  ;[1 0.8122 0] CreateDefaultName
  (Rendering|Components|TextRender|SetText (Variables|Default|GetTextRender) (Utilities|Text|ToText(String) (Utilities|String|Append "Team" (Utilities|String|ToString(Byte) (Variables|Default|GetTeamID)) "_" "Player" (Utilities|String|ToString(Integer) NumberInTeam))))
  (if (== (Variables|Default|GetTeamID) 1)
    (Rendering|Components|TextRender|SetTextRenderColor (Variables|Default|GetTextRender) (Math|Color|MakeColor 0 0 255 255))
    (else
      (Rendering|Components|TextRender|SetTextRenderColor (Variables|Default|GetTextRender) (Math|Color|MakeColor 255 0 0 255)))))

(event Custom|Server_TakeDamage
  (params (Damage :type Float%20%28single-precision%29) (MultiPawn :type BP%20Multiplayer%20Pawn%20Object%20Reference))
  (bind _healthcomponent (Variables|BP_MultiplayerPawn_C|GetHealthComponent MultiPawn))
  ;[1 1 1] Damage
  (Variables|/Game/MyContent/BP/HealthComponent.HealthComponent_C|SetCurrentHEalth _healthcomponent (- (Variables|/Game/MyContent/BP/HealthComponent.HealthComponent_C|GetCurrentHEalth _healthcomponent) Damage)))

(event Custom|Reload
  ;[1 1 1] Отрабатывает если играть от лица сервера.
  ;;[1 0 0] Задержка выстрела
  (Variables|Default|SetCanFire false)
  (Utilities|FlowControl|Delay 1.0)
  (Variables|Default|SetCanFire true))

(event Custom|CreateHealthWidgetOnViewport
  (bind _healthcomponent (Variables|Default|GetHealthComponent))
  ;[1 0 0] Обновление хелзбара при старте
  (bind _returnvalue (UserInterface|CreateWidget "/Game/MyContent/Wdgets/WBP_HealthWidget.WBP_HealthWidget_C" (Game|GetPlayerController 0)))
  (bind _output_get (Variables|Default|SetHealthWidget _returnvalue))
  (UserInterface|Viewport|AddtoViewport _output_get 0)
  (Progress|SetPercent (Variables|/Game/MyContent/Wdgets/WBP_HealthWidget.WBP_HealthWidget_C|GetHealthbar (Variables|Default|GetHealthWidget)) (/ (Variables|/Game/MyContent/BP/HealthComponent.HealthComponent_C|GetCurrentHEalth _healthcomponent) (Variables|/Game/MyContent/BP/HealthComponent.HealthComponent_C|GetMaxHealth _healthcomponent))))

(event Custom|Set%20MaterialByTeam
  (bind _teamid (Variables|Default|GetTeamID))
  (if (== _teamid 1)
    (Rendering|Material|SetMaterial (Variables|Default|GetSphere) 0 "/Game/StarterContent/Materials/M_Tech_Hex_Tile.M_Tech_Hex_Tile")
    (elif (== 2 _teamid)
      (Rendering|Material|SetMaterial (Variables|Default|GetSphere) 0 "/Game/StarterContent/Materials/M_Tech_Hex_Tile_Pulse.M_Tech_Hex_Tile_Pulse"))))

(event Custom|Server_SetTEamID
  (params (TeamID :type Byte) (PlayerNumber :type Integer))
  (Variables|Default|SetTeamID TeamID)
  (CallFunction|MulticastChangedTeamID))

(event Custom|Server_ChagedTeamID
  (CallFunction|MulticastChangedTeamID))

(event Custom|Multicast_ChangedTeamID
  (CallFunction|SetMaterialbyTeam))

(event EventBeginPlay
  ;[0.1408 1 0] BeginPlay
  (bind _asbp_multiplayer_player_controller (Utilities|Casting|CastToBP_MultiplayerPlayerController (Pawn|GetController))
    (:then
      (CallFunction|ServerSetTEamID (Variables|/Game/MyContent/BP/BP_MultiplayerPlayerController.BP_MultiplayerPlayerController_C|GetTeamID _asbp_multiplayer_player_controller)))
    (:CastFailed
      (CallFunction|SetMaterialbyTeam))))

(event Collision|EventActorBeginOverlap
  (params (OtherActor :type Actor%20Object%20Reference)))

(event EventTick
  (params (DeltaSeconds :type Float%20%28single-precision%29))
  ;[1 1 1] Destroy Actor
  (if (<= (Variables|/Game/MyContent/BP/HealthComponent.HealthComponent_C|GetCurrentHEalth (Variables|Default|GetHealthComponent)) 0.0)
    (Actor|DestroyActor)
    (Widget|RemovefromParent (Variables|Default|GetHealthWidget))))

(event Input|ActionEvents|InputActionJump
  (params (Key :type Key%20Structure :default "None"))
  ;[1 1 1] Movement/Rotation
  (:Pressed
    (Character|Jump))
  (:Released
    (Character|StopJumping)))

(event Input|AxisEvents|InputAxisLookUp
  (params (AxisValue :type Float%20%28single-precision%29))
  ;[1 1 1] Movement/Rotation
  (Pawn|Input|AddControllerPitchInput AxisValue))

(event Input|AxisEvents|InputAxisTurn
  (params (AxisValue :type Float%20%28single-precision%29))
  ;[1 1 1] Movement/Rotation
  (Pawn|Input|AddControllerYawInput AxisValue))

(event Input|AxisEvents|InputAxisMoveForward
  (params (AxisValue :type Float%20%28single-precision%29))
  ;[1 1 1] Movement/Rotation
  (Pawn|Input|AddMovementInput (Math|Vector|GetForwardVector (Math|Rotator|MakeRotator 0.0 0.0 (.yaw (Pawn|GetControlRotation :!class /Script/Engine.Pawn)))) AxisValue false))

(event Input|AxisEvents|InputAxisMoveRight
  (params (AxisValue :type Float%20%28single-precision%29))
  ;[1 1 1] Movement/Rotation
  (Pawn|Input|AddMovementInput (Math|Vector|GetRightVector (Math|Rotator|MakeRotator 0.0 0.0 (.yaw (Pawn|GetControlRotation :!class /Script/Engine.Pawn)))) AxisValue false))

(event Input|MouseEvents|LeftMouseButton
  (params (Key :type Key%20Structure :default "None"))
  ;[1 1 1] Fire
  (:Pressed
    (CallFunction|ServerFire)))

(event Input|KeyboardEvents|Tab
  (params (Key :type Key%20Structure :default "None"))
  (:Pressed
    (bind _asbp_multiplayer_game_mode (Utilities|Casting|CastToBP_MultiplayerGameMode (Game|GetGameMode)))
    (for _array_element (Variables|/Game/MyContent/BP/BP_MultiplayerGameMode.BP_MultiplayerGameMode_C|GetTeam1 _asbp_multiplayer_game_mode)
      (Development|PrintString (Utilities|String|Append "Team 1: " (Utilities|GetDisplayName _array_element)) true true "(R=0.000000,G=0.057792,B=0.619792,A=1.000000)" 6e+01)
      (for _array_element_2 (Variables|/Game/MyContent/BP/BP_MultiplayerGameMode.BP_MultiplayerGameMode_C|GetTeam2 _asbp_multiplayer_game_mode)
        (Development|PrintString (Utilities|String|Append "Team 2: " (Utilities|GetDisplayName _array_element_2)) true true "(R=1.000000,G=0.000000,B=0.000000,A=1.000000)" 6e+01)))))

(event Input|KeyboardEvents|1
  (params (Key :type Key%20Structure :default "None"))
  (bind _returnvalue (Game|GetPlayerController 0))
  (:Pressed
    (Utilities|FlowControl|FlipFlop
      (:A
        (bind _returnvalue_2 (UserInterface|CreateWidget "/Game/MyContent/Wdgets/WBP_Pause.WBP_Pause_C" _returnvalue))
        (bind _output_get (Variables|Default|SetPauseWidget _returnvalue_2))
        (UserInterface|Viewport|AddtoViewport _output_get 0)
        (Variables|/Script/Engine.PlayerController|SetbShowMouseCursor _returnvalue true)
        (Pawn|UnPossess _returnvalue)))))

(fn ConstructionScript)